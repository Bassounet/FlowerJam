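; BP_Drop is a falling drop actor that turns into a BP_Gatling when it lands.
; On BeginPlay the slowed Descente timeline lerps the StaticMesh's relative Z from the actor's current height toward a fixed low height.
; Once the actor's Z falls below a threshold, Landee stops the timeline, spawns the gatling at a height offset from the Sphere's relative Z, and destroys the drop.
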(event `self.ReceiveBeginPlay`
  (bind (_returnvalue_x _returnvalue_y _returnvalue_z) (`KismetMathLibrary.BreakVector` (`self.K2_GetActorLocation`)))
  (`TimelineComponent.SetPlayRate` (`self.Descente`) 0.006)
  (bind (_direction _newtrack_0) (`Timeline|Descente` :!via `PlayFromStart`)
    (:`Update`
      (if (not (< _returnvalue_z 220.0))
        (`SceneComponent.K2_SetRelativeLocation` (`self.StaticMesh`) (`KismetMathLibrary.MakeVector` 0.0 0.0 (`KismetMathLibrary.Lerp` _returnvalue_z 200.0 _newtrack_0)) false false)
        (else
          (`KismetSystemLibrary.PrintString` "Hello")
          (`self.Landee`))))))

(event `Landee`
  (bind (_relativelocation_x _relativelocation_y _relativelocation_z) (`KismetMathLibrary.BreakVector` (`SceneComponent.RelativeLocation` (`self.Sphere`))))
  (`TimelineComponent.Stop` (`self.Descente`))
  (`|SpawnActorFromClass` "/Game/PureBP/BP_Gatling.BP_Gatling_C" (`KismetMathLibrary.MakeTransform` (`KismetMathLibrary.MakeVector` 0.0 0.0 (+ _relativelocation_z 250.0))) "Undefined" "OverrideRootScale" null null)
  (`self.K2_DestroyActor`))

(fn `UserConstructionScript`)