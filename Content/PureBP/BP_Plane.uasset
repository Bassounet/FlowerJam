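; BP_Plane is a plane actor that flies along world Y while repeatedly releasing pairs of missiles.
; A slowed MoveForward timeline drives movement, lerping from the current location each update, so displacement accumulates rather than following a fixed path.
; A looping timer fires Largage, spawning a BP_Missile at each of two box components and calling LargageMissile on both.
; A stepped, wrapping Y offset staggers spawn points and is printed for debugging.
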(event `self.ReceiveBeginPlay`
  (bind (_returnvalue_x _returnvalue_y _returnvalue_z) (`KismetMathLibrary.BreakVector` (`self.K2_GetActorLocation`)))
  (`KismetSystemLibrary.K2_SetTimerDelegate` (delegate `Largage`) 0.2 true)
  (`TimelineComponent.SetPlayRate` (`self.MoveForward`) 0.1)
  (bind (_direction _mouveforward) (`Timeline|MoveForward` :!via `PlayFromStart`)
    (:`Update`
      (`self.K2_SetActorLocation` (`KismetMathLibrary.MakeVector` _returnvalue_x (`KismetMathLibrary.Lerp` _returnvalue_y (+ _returnvalue_y (`self.DistanceGoThrought`)) _mouveforward) _returnvalue_z)))))

(event `Largage`
  (if (>= (`self.Offset`) 2200.0)
    (set `self.Offset` 0.0))
  (bind _returnvalue (`|SpawnActorFromClass` "/Game/PureBP/BP_Missile.BP_Missile_C" (`KismetMathLibrary.MakeTransform` (+ (`SceneComponent.K2_GetComponentLocation` (`self.Box1`)) (`KismetMathLibrary.MakeVector` 0.0 (`self.Offset`)))) "Undefined" "OverrideRootScale" null null))
  (bind _returnvalue_2 (`|SpawnActorFromClass` "/Game/PureBP/BP_Missile.BP_Missile_C" (`KismetMathLibrary.MakeTransform` (+ (`SceneComponent.K2_GetComponentLocation` (`self.Box`)) (`KismetMathLibrary.MakeVector` 0.0 (`self.Offset`)))) "Undefined" "OverrideRootScale" null null))
  (`/Game/PureBP/BP_Missile.LargageMissile` _returnvalue)
  (`/Game/PureBP/BP_Missile.LargageMissile` _returnvalue_2)
  (bind _output_get (set `self.Offset` (+ (`self.Offset`) 300.0)))
  (`KismetSystemLibrary.PrintString` (`KismetStringLibrary.Conv_DoubleToString` _output_get)))

(fn `UserConstructionScript`)