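; BP_Missile is a missile actor that can be launched or released and marks a danger zone as it descends.
; LaunchMissile adds a projectile movement component at runtime with a forward local velocity, while LargageMissile adds one without setting velocity.
; Tick calls DangerIncomming whenever vertical velocity is below a small threshold.
; That shows DangerZone at the missile's XY position, scaled inversely with missile height and clamped, so it grows as the missile nears zero height.
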(event `self.ReceiveTick`
  (params (DeltaSeconds :type "Float (single-precision)"))
  (bind (_returnvalue_x _returnvalue_y _returnvalue_z) (`KismetMathLibrary.BreakVector` (`self.GetVelocity`)))
  (if (< _returnvalue_z 50.0)
    (`self.DangerIncomming`)))

(event `DangerIncomming`
  (bind (_returnvalue_x _returnvalue_y) (`KismetMathLibrary.BreakVector` (`self.K2_GetActorLocation`)))
  (bind (_returnvalue_x_2 _returnvalue_y_2 _returnvalue_z) (`KismetMathLibrary.BreakVector` (`SceneComponent.K2_GetComponentLocation` (`self.Missile`))))
  (`SceneComponent.SetVisibility` (`self.DangerZone`) true false)
  (`SceneComponent.K2_SetWorldLocation` (`self.DangerZone`) (`KismetMathLibrary.MakeVector` _returnvalue_x _returnvalue_y) false false)
  (`SceneComponent.SetWorldScale3D` (`self.DangerZone`) (`KismetMathLibrary.ClampVectorSize` (/ 1.0 (/ (`KismetMathLibrary.Conv_DoubleToVector` _returnvalue_z) 1000.0)) 0.0 20.0)))

(event `self.ReceiveBeginPlay`)

(event `LaunchMissile`
  (params (`Initial Speed` :type "Float (single-precision)"))
  (bind _returnvalue (`AddComponent|NODE_AddProjectileMovementComponent-1`))
  (`ProjectileMovementComponent.SetVelocityInLocalSpace` _returnvalue (`KismetMathLibrary.MakeVector` `Initial Speed`)))

(event `LargageMissile`
  (`AddComponent|NODE_AddProjectileMovementComponent-2`))

(fn `UserConstructionScript`)