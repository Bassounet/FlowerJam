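; BP_FlowerProjectile is a projectile actor with projectile and rotating movement that expires five seconds after spawning.
; On hit it stops both movements, sets projectile gravity scale to normal and prints debug text.
; It casts the hit actor to the player character and the enemy.
; An enemy hit calls MessageMessage on the character cast result, taken from that same actor; other hits print an environment message.
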(event `self.ReceiveBeginPlay`
  (`self.SetLifeSpan` 5.0))

(event `self.ReceiveHit`
  (params (MyComp :type "PrimitiveComponent Object Reference") (Other :type "Actor Object Reference") (OtherComp :type "PrimitiveComponent Object Reference") (bSelfMoved :type Boolean) (HitLocation :type "Vector Structure") (HitNormal :type "Vector Structure") (NormalImpulse :type "Vector Structure") (Hit :type "HitResult Structure (by ref)"))
  (bind _projectilemovement (`self.ProjectileMovement`))
  (`KismetSystemLibrary.PrintString` "aaaaaHello")
  (`MovementComponent.StopMovementImmediately` _projectilemovement)
  (`MovementComponent.StopMovementImmediately` (`self.RotatingMovement`))
  (set `ProjectileMovementComponent.ProjectileGravityScale` 1.0 _projectilemovement)
  (bind _asbp_third_person_character (cast `/Game/ThirdPerson/Blueprints/BP_ThirdPersonCharacter` Other)
    (:`then`
      _)
    (:`CastFailed`
      _))
  (cast `/Game/PureBP/BP_Ennemy` Other
    (:`then`
      (message `/Game/PureBP/BPI_Message.Message` _asbp_third_person_character))
    (:`CastFailed`
      (`KismetSystemLibrary.PrintString` "Projectil_Hitting_Environment"))))

(fn `UserConstructionScript`)