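; BP_Helico is a helicopter actor that flies along negative Y with spinning rotors, then despawns.
; On BeginPlay, a slowed MoveForward timeline offsets its location while a slowed Rotate timeline spins the main rotor in yaw and tail rotor in roll, both lerping from current values each update.
; Rotate restarts itself through Turn on finish; its first completion also sets Launched and starts the TimeBeforeDesappear delay before DestroyActor.
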(event `self.ReceiveBeginPlay`
  (bind _helicecentrale (`self.HeliceCentrale`))
  (bind _helicearr (`self.HeliceArr`))
  (bind _relativerotation_roll (`KismetMathLibrary.BreakRotator` (`SceneComponent.RelativeRotation` _helicearr)))
  (bind (_relativerotation_roll_2 _relativerotation_pitch _relativerotation_yaw) (`KismetMathLibrary.BreakRotator` (`SceneComponent.RelativeRotation` _helicecentrale)))
  (`TimelineComponent.SetPlayRate` (`self.Rotate`) 0.001)
  (`self.GoForwarrd`)
  (bind (_direction _newtrack_0) (`Timeline|Rotate` :!via `PlayFromStart` :!label _label)
    (:`Update`
      (bind (_returnvalue_x _returnvalue_y) (`KismetMathLibrary.BreakVector` (`KismetMathLibrary.VLerp` (`KismetMathLibrary.Conv_DoubleToVector` _relativerotation_yaw) (`KismetMathLibrary.Conv_DoubleToVector` (+ _relativerotation_yaw 10000.0)) _newtrack_0)))
      (`SceneComponent.K2_SetRelativeRotation` _helicecentrale (`KismetMathLibrary.MakeRotator` 0.0 0.0 _returnvalue_y) false false)
      (bind _returnvalue_x_2 (`KismetMathLibrary.BreakVector` (`KismetMathLibrary.VLerp` (`KismetMathLibrary.Conv_DoubleToVector` _relativerotation_roll) (`KismetMathLibrary.Conv_DoubleToVector` (+ _relativerotation_roll 10000.0)) _newtrack_0)))
      (`SceneComponent.K2_SetRelativeRotation` _helicearr (`KismetMathLibrary.MakeRotator` _returnvalue_x_2) false false))
    (:`Finished`
      (if (`self.Launched?`)
        (`self.Turn`)
        (else
          (`self.Turn`)
          (set `self.Launched?` true)
          (`KismetSystemLibrary.Delay` (`self.TimeBeforeDesappear`))
          (`self.K2_DestroyActor`))))))

(event `Turn`
  (goto _label :!via `PlayFromStart`))

(event `GoForwarrd`
  (bind _returnvalue (`self.K2_GetActorLocation`))
  (`TimelineComponent.SetPlayRate` (`self.MoveForward`) 0.01)
  (bind (_direction _newtrack_0) (`Timeline|MoveForward` :!via `PlayFromStart`)
    (:`Update`
      (`self.K2_SetActorLocation` (`KismetMathLibrary.VLerp` _returnvalue (+ _returnvalue (0.0 -1000.0 0.0)) _newtrack_0)))))

(fn `UserConstructionScript`)