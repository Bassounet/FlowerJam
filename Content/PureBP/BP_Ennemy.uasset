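; Patrolling AI gunman that, when hit, turns peaceful, charges the player's ult and dances.
; BeginPlay builds a faction-based (Viet or US) list of shot sounds and starts its behavior tree; construction turns spline points into patrol locations.
; Fire starts a looping timer that spawns randomly angled bullets until hit.
; Message handles the hit: it sets the "Peace?" blackboard key, then chains death, gun drop, getting-up and looping Gangnam Style montages.
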(event `self.ReceiveBeginPlay`
  (`|ExecutionSequence`
    (:`then_0`
      ;[0.8879 1 0.07619] CreateList
      (bind _output_get (set `self.ShootCuesList` (`|MakeArray` (`self.Balle_Cue`) (`self.Balle_Cue`) (`self.Balle_Cue`) (`self.Balle_Cue`) (`self.Balle_Cue`) (`self.Balle_Cue`))))
      (if (`self.isChingChong?`)
        (for _array_element (`|MakeArray` (`self.VietBullet1_Cue`) (`self.VietBullet2_Cue`) (`self.VietBullet3_Cue`))
          (`KismetArrayLibrary.Array_Add` _output_get _array_element))
        (else
          (for _array_element_2 (`|MakeArray` (`self.UsBullet2_Cue`) (`self.UsBullet1_Cue`) (`self.UsBullet3_Cue`))
            (`KismetArrayLibrary.Array_Add` _output_get _array_element_2)))))
    (:`then_1`
      ;[0 0.01677 1] Begin
      (bind _asaic_ennemy (cast `/Game/PureBP/AIC_Ennemy` (`AIBlueprintHelperLibrary.GetAIController` self)))
      (`/Game/PureBP/AIC_Ennemy.SetupAIC` _asaic_ennemy (`self.BehaviorTree`))
      (set `self.REF_OriginEnnemy` (`self.K2_GetActorLocation`)))))

(event `Fire`
  ;[0 1 0.02047] Shoot
  (if (and (not (`self.HasBeenHit`)) (`self.ShootingByDefault`))
    _
    (else
      _))
  (bind _returnvalue (`KismetSystemLibrary.K2_SetTimerDelegate` (delegate `Shoot`) 0.5 true))
  (set `self.REF_TimerFaya` _returnvalue))

(event `Shoot`
  (bind (_returnvalue_roll _returnvalue_pitch _returnvalue_yaw) (`KismetMathLibrary.BreakRotator` (`KismetMathLibrary.Conv_VectorToRotator` (`SceneComponent.GetForwardVector` (`self.Mesh`)))))
  (bind _returnvalue (+ _returnvalue_yaw 90.0))
  ;[0 1 0.02047] Shoot
  (if (not (`self.HasBeenHit`))
    (`|SpawnActorFromClass` "/Game/PureBP/BP_Bullet.BP_Bullet_C" (`KismetMathLibrary.MakeTransform` (+ (`SceneComponent.K2_GetComponentLocation` (`self.muzzle`)) (`KismetMathLibrary.GreaterGreater_VectorRotator` (0.0 0.0 0.0) (`KismetMathLibrary.MakeRotator` _returnvalue_roll _returnvalue_pitch _returnvalue_yaw))) (`KismetMathLibrary.MakeRotator` 0.0 (`KismetMathLibrary.RandomFloatInRange` -10.0 10.0) (`KismetMathLibrary.RandomFloatInRange` _returnvalue (+ _returnvalue 30.0))) (0.4 0.4 0.4)) "Undefined" "OverrideRootScale" null null)
    ;[0.8879 1 0.07619] Play Sound
    (`GameplayStatics.PlaySoundAtLocation` (`AudioComponent.Sound` (`KismetArrayLibrary.Array_Random` (`self.ShootCuesList`))) (`SceneComponent.K2_GetComponentLocation` (`self.Mesh`)) (struct) 1.0 1.0 0.0 null null null null)))

(event `/Game/PureBP/BPI_Message.Message`
  (bind _mesh (`self.Mesh`))
  (if (not (`self.HasBeenHit`))
    (bind _returnvalue (`GameplayStatics.GetActorOfClass` "/Game/ThirdPerson/Blueprints/BP_ThirdPersonCharacter.BP_ThirdPersonCharacter_C"))
    (`/Game/ThirdPerson/Blueprints/BP_ThirdPersonCharacter.ChargeUlt` _returnvalue)
    (set `self.HasBeenHit` true)
    (`/Game/PureBP/BP_Library.UpdateBBKey` "NewEnumerator0" (`AIBlueprintHelperLibrary.GetAIController` self) "Peace?" true)
    (`|PlayMontage` _mesh "/Game/3D/Animation/Soldier/Death_Montage.Death_Montage"
      (:`OnBlendOut`
        (`SceneComponent.K2_DetachFromComponent` (`self.gun`) "KeepRelative" "KeepRelative" "KeepRelative" true)
        (`|PlayMontage` _mesh "/Game/3D/Animation/Soldier/Getting_Up_Montage.Getting_Up_Montage"
          (:`OnCompleted`
            (`|PlayMontage` _mesh "/Game/3D/Animation/Soldier/Gangnam_Style_Montage.Gangnam_Style_Montage" :!label _label
              (:`OnBlendOut`
                (goto _label)))))))))

(fn `UserConstructionScript`
  (`KismetArrayLibrary.Array_Clear` (`self.PatrolPoints`))
  (for _index (range (+ (`SplineComponent.GetNumberOfSplinePoints` (`self.SplinePatrolPoints`)) 1))
    (`KismetArrayLibrary.Array_Add` (`self.PatrolPoints`) (`SplineComponent.GetLocationAtSplinePoint` (`self.SplinePatrolPoints`) _index "World"))))