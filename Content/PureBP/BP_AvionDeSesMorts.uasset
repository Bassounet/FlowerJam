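; Bomber plane actor that flies along its mesh's forward vector while continuously dropping missiles.
; On BeginPlay, a timeline moves the root by lerping from the mesh's current location, re-read each update, toward a point ahead.
; A fast looping timer spawns BP_Missile pairs at two box components and calls LargageMissile on them.
; Each drop steps a world-X offset backward, wrapping to zero past a limit and printing it for debug.
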(event `self.ReceiveBeginPlay`
  (bind _staticmesh (`self.StaticMesh`))
  (bind _returnvalue (`SceneComponent.K2_GetComponentLocation` _staticmesh))
  (`KismetSystemLibrary.K2_SetTimerDelegate` (delegate `CustomEvent_0`) 0.1 true)
  (`TimelineComponent.SetPlayRate` (`self.Timeline_0`) 0.01)
  (bind (_direction _newtrack_0) (`Timeline|Timeline_0` :!via `PlayFromStart`)
    (:`Update`
      (`SceneComponent.K2_SetWorldLocation` (`self.DefaultSceneRoot`) (`KismetMathLibrary.VLerp` _returnvalue (+ _returnvalue (* (`SceneComponent.GetForwardVector` _staticmesh) (`self.NewVar_0`))) _newtrack_0) false false))))

(event `CustomEvent_0`
  (if (not (>= (`self.Offset`) -2200.0))
    (set `self.Offset` 0.0))
  (bind _returnvalue (`|SpawnActorFromClass` "/Game/PureBP/BP_Missile.BP_Missile_C" (`KismetMathLibrary.MakeTransform` (+ (`SceneComponent.K2_GetComponentLocation` (`self.Box`)) (`KismetMathLibrary.MakeVector` (`self.Offset`))) (struct) (3.0 3.0 3.0)) "Undefined" "OverrideRootScale" null null))
  (bind _returnvalue_2 (`|SpawnActorFromClass` "/Game/PureBP/BP_Missile.BP_Missile_C" (`KismetMathLibrary.MakeTransform` (+ (`SceneComponent.K2_GetComponentLocation` (`self.Box1`)) (`KismetMathLibrary.MakeVector` (`self.Offset`))) (struct) (3.0 3.0 3.0)) "Undefined" "OverrideRootScale" null null))
  (`/Game/PureBP/BP_Missile.LargageMissile` _returnvalue)
  (`/Game/PureBP/BP_Missile.LargageMissile` _returnvalue_2)
  (bind _output_get (set `self.Offset` (+ (`self.Offset`) -150.0)))
  (`KismetSystemLibrary.PrintString` (`KismetStringLibrary.Conv_DoubleToString` _output_get)))

(fn `UserConstructionScript`)