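; BP_Mortar is a mortar actor that starts firing automatically on BeginPlay and keeps launching BP_Missile projectiles.
; Fire stores a looping one-second timer that calls Shoot.
; Shoot spawns each missile at a rotated offset from component W, taking yaw from W's forward vector and randomizing pitch within a steep upward range for a lobbed launch angle.
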(event `self.ReceiveBeginPlay`
  (`self.Fire`))

(event `Fire`
  (bind _returnvalue (`KismetSystemLibrary.K2_SetTimerDelegate` (delegate `Shoot`) 1.0 true))
  (set `self.REF` _returnvalue))

(event `Shoot`
  (bind (_returnvalue_roll _returnvalue_pitch _returnvalue_yaw) (`KismetMathLibrary.BreakRotator` (`KismetMathLibrary.Conv_VectorToRotator` (`SceneComponent.GetForwardVector` (`self.w`)))))
  (`|SpawnActorFromClass` "/Game/PureBP/BP_Missile.BP_Missile_C" (`KismetMathLibrary.MakeTransform` (+ (`SceneComponent.K2_GetComponentLocation` (`self.w`)) (`KismetMathLibrary.GreaterGreater_VectorRotator` (0.0 0.0 0.0) (`KismetMathLibrary.MakeRotator` _returnvalue_roll _returnvalue_pitch _returnvalue_yaw))) (`KismetMathLibrary.MakeRotator` 0.0 (`KismetMathLibrary.RandomFloatInRange` 50.0 60.0) _returnvalue_yaw)) "Undefined" "OverrideRootScale" null null))

(fn `UserConstructionScript`)